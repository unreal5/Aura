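; Gameplay ability that casts a Fire Bolt projectile at the location under the mouse.
; On activation it takes the hit location from mouse target data, sends the avatar a facing-target interface message and plays the cast montage.
; A gameplay event from the montage triggers the projectile spawn toward that location.
; The ability ends on montage completion rather than at spawn, so spawning does not cancel it.
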(event `self.K2_ActivateAbility`
  (bind (_asynctaskproxy _targetdatahandle) (`TargetDataUnderMouse.CreateTargetDataUnderMouse`)
    (:`ValidData`
      (set `self.ProjectileTargetLocation` (`.Location` (`GameplayStatics.BreakHitResult` (`AbilitySystemBlueprintLibrary.GetHitResultFromTargetData` _targetdatahandle))))
      ;[1 1 1] 对于右上角有信封的，意思是如果没有实现对应的接口，则什么也不做。
      (message `CombatInterface.UpdateFacingTarget` (`self.GetAvatarActorFromActorInfo`) (`self.ProjectileTargetLocation`))
      (`AbilityTask_PlayMontageAndWait.CreatePlayMontageAndWaitProxy` "None" "/Game/Assets/Characters/Aura/Animations/Abilities/AM_Cast_FireBolt.AM_Cast_FireBolt"
        (:`then`
          (`AbilityTask_WaitGameplayEvent.WaitGameplayEvent` (struct :`TagName` "Event.Montage.FireBolt") null
            (:`EventReceived`
              (`self.SpawnProjectile` (`self.ProjectileTargetLocation`)))))
        (:`OnCompleted`
          (`self.K2_EndAbility`))))))