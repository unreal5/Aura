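; Melee attack gameplay ability that turns the avatar toward its combat target and damages nearby live players.
; It plays a random attack montage from the avatar's interface and waits for that attack's gameplay event tag.
; On the event, it damages others within a small radius of the tagged combat socket, then ends.
; The random index is drawn separately for montage, event tag and socket, so they can mismatch.
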(event `self.K2_ActivateAbility`
  (bind _returnvalue (`self.GetAvatarActorFromActorInfo`))
  (bind _returnvalue_2 (`self.GetAvatarActorFromActorInfo`))
  (bind _returnvalue_3 (message `EnemyInterface.GetCombatTarget` _returnvalue_2))
  (`/Engine/EditorBlueprintResources/StandardMacros.IsValid` _returnvalue_3
    (:`Is Valid`
      (message `CombatInterface.UpdateFacingTarget` _returnvalue_2 (`Actor.K2_GetActorLocation` _returnvalue_3))
      (bind _returnvalue_4 (message `CombatInterface.GetAttackMontages` _returnvalue_2))
      (bind (_montage _montagetag) (break `TaggedMontage` (`|GetArrayItem` _returnvalue_4 (`KismetMathLibrary.RandomIntegerInRange` 0 (- (`KismetArrayLibrary.Array_Length` _returnvalue_4) 1)))))
      (`AbilityTask_PlayMontageAndWait.CreatePlayMontageAndWaitProxy` "None" _montage
        (:`then`
          (`AbilityTask_WaitGameplayEvent.WaitGameplayEvent` _montagetag null
            (:`EventReceived`
              (bind _returnvalue_5 (message `CombatInterface.GetCombatSocketLocation` _returnvalue _montagetag))
              (bind _outoverlappingactors (`AuraAbilitySystemLibrary.GetLivePlayersWithinRadius` self (`|MakeArray` _returnvalue) _returnvalue_5 45.0))
              (for _array_element _outoverlappingactors
                (`self.CauseDamage` _array_element))
              (`self.K2_EndAbility`))))))))