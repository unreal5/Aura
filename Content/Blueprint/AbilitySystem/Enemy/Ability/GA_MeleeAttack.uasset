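; Enemy melee attack ability that turns the avatar toward its combat target and plays a random tagged attack montage.
; Avatar interface calls supply the target, montages and combat socket location.
; The montage's tag doubles as the awaited gameplay event and socket selector; on that event, non-friendly live players in a small radius there take damage.
; The ability then ends without stopping the montage, or ends when the montage completes or is interrupted.
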(event `self.K2_ActivateAbility`
  (bind _returnvalue (`self.GetAvatarActorFromActorInfo`))
  (bind _returnvalue_2 (`self.GetAvatarActorFromActorInfo`))
  (bind _returnvalue_3 (message `EnemyInterface.GetCombatTarget` _returnvalue_2))
  (`/Engine/EditorBlueprintResources/StandardMacros.IsValid` _returnvalue_3
    (:`Is Valid`
      (message `CombatInterface.UpdateFacingTarget` _returnvalue_2 (`Actor.K2_GetActorLocation` _returnvalue_3))
      (bind _returnvalue_4 (message `CombatInterface.GetAttackMontages` _returnvalue_2))
      (bind _output_get (set `self.TaggedMontage` (`self.GetRandomTaggedMontageFromArray` _returnvalue_4)))
      (bind (_montage _montagetag) (break `TaggedMontage` _output_get))
      (`AbilityTask_PlayMontageAndWait.CreatePlayMontageAndWaitProxy` "None" _montage 1.0 "None" false
        (:`then`
          (`AbilityTask_WaitGameplayEvent.WaitGameplayEvent` _montagetag null
            (:`EventReceived`
              (bind _returnvalue_5 (message `CombatInterface.GetCombatSocketLocation` _returnvalue _montagetag))
              (bind _outoverlappingactors (`AuraAbilitySystemLibrary.GetLivePlayersWithinRadius` self (`|MakeArray` _returnvalue) _returnvalue_5 45.0))
              (for _array_element _outoverlappingactors
                (if (`AuraAbilitySystemLibrary.IsNotFriendly` (`self.GetAvatarActorFromActorInfo`) _array_element)
                  (`self.CauseDamage` _array_element)))
              (`self.K2_EndAbility`))))
        (:`OnCompleted`
          (`self.K2_EndAbility` :!label _label))
        (:`OnInterrupted`
          (goto _label))
        (:`OnCancelled`
          (goto _label))))))