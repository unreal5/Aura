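; GA_RangedAttack is an enemy gameplay ability that performs a ranged attack on the avatar's combat target.
; It turns the avatar toward the target, plays a random tagged attack montage, and waits for the gameplay event matching that montage's tag.
; On that event it looks up the socket location and spawns a projectile aimed at the target's current position.
; The ability ends when the montage completes, is interrupted or is cancelled.
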(event `self.K2_ActivateAbility`
  (bind _returnvalue (`self.GetAvatarActorFromActorInfo`))
  (bind _returnvalue_2 (message `EnemyInterface.GetCombatTarget` _returnvalue))
  (`/Engine/EditorBlueprintResources/StandardMacros.IsValid` _returnvalue_2
    (:`Is Valid`
      (message `CombatInterface.UpdateFacingTarget` _returnvalue (`Actor.K2_GetActorLocation` _returnvalue_2))
      (bind _returnvalue_3 (message `CombatInterface.GetAttackMontages` _returnvalue))
      (bind _output_get (set `self.TaggedMontage` (`self.GetRandomTaggedMontageFromArray` _returnvalue_3)))
      (`AbilityTask_PlayMontageAndWait.CreatePlayMontageAndWaitProxy` "None" (break `TaggedMontage` _output_get) 1.0 "None" false
        (:`then`
          (`AbilityTask_WaitGameplayEvent.WaitGameplayEvent` (`.MontageTag` (break `TaggedMontage` _output_get)) null
            (:`EventReceived`
              (message `CombatInterface.GetCombatSocketLocation` (`self.GetAvatarActorFromActorInfo`) (`.SocketTag` (break `TaggedMontage` _output_get)))
              (bind _returnvalue_4 (message `EnemyInterface.GetCombatTarget` (`self.GetAvatarActorFromActorInfo`)))
              (`self.SpawnProjectile` (`Actor.K2_GetActorLocation` _returnvalue_4)))))
        (:`OnCompleted`
          (`self.K2_EndAbility` :!label _label))
        (:`OnInterrupted`
          (goto _label))
        (:`OnCancelled`
          (goto _label))))))