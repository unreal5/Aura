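; GA_Summon is an enemy gameplay ability for summoning, currently previewing spawn points with debug spheres rather than spawning anything.
; On activation the avatar turns toward its combat target, then the ability fetches spawn locations and shuffles them.
; A looped Delay steps through the locations one per second, drawing a sphere at each, and ends the ability after the last.
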(event `self.K2_ActivateAbility`
  (bind _returnvalue (`self.GetAvatarActorFromActorInfo`))
  (bind _returnvalue_2 (message `EnemyInterface.GetCombatTarget` _returnvalue))
  (message `CombatInterface.UpdateFacingTarget` _returnvalue (`Actor.K2_GetActorLocation` _returnvalue_2))
  (bind _returnvalue_3 (`self.GetSpawnLocations`))
  (bind _output_get (set `self.SpawnLocations` _returnvalue_3))
  (`KismetArrayLibrary.Array_Shuffle` _output_get)
  (if (< (`self.SpawnLocationIndex`) (`KismetArrayLibrary.Array_Length` (`self.SpawnLocations`))) :!label _label
    (`KismetSystemLibrary.DrawDebugSphere` (`|GetArrayItem` (`self.SpawnLocations`) (`self.SpawnLocationIndex`)) 25.0 12 (struct :`R` 1.0 :`G` 0.829104 :`B` 0.083333 :`A` 1.0) 3.0 2.0)
    (`/Engine/EditorBlueprintResources/StandardMacros.IncrementInt` (`self.SpawnLocationIndex`)
      (:`  `
        (`KismetSystemLibrary.Delay` 1.0)
        (goto _label)))
    (else
      (`self.K2_EndAbility`))))