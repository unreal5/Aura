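; GA_FireBolt is the Fire Bolt gameplay ability, which casts a projectile through an animation montage.
; On activation it gets target data under the mouse, draws a randomly colored debug sphere there, then plays the cast montage.
; A one-time wait for the montage's gameplay event triggers SpawnProjectile with an identity transform; the target data feeds only the debug sphere.
; The ability ends when the montage completes, is interrupted or is cancelled.
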(event `self.K2_ActivateAbility`
  (bind (_asynctaskproxy _targetdata) (`TargetDataUnderMouse.CreateTargetDataUnderMouse` "TargetDataUnderMouse")
    (:`OnTargetDataReady`
      (`KismetSystemLibrary.DrawDebugSphere` _targetdata 50.0 12 (make `LinearColor` (`KismetMathLibrary.RandomFloatInRange` 0.0 1.0) (`KismetMathLibrary.RandomFloatInRange` 0.0 1.0) (`KismetMathLibrary.RandomFloatInRange` 0.0 1.0) 1.0) 2.0 1.0)
      (`AbilityTask_PlayMontageAndWait.CreatePlayMontageAndWaitProxy` "None" "/Game/Blueprints/AbilitySystem/GameplayAbility/Fire/FireBolt/Montage/AM_Cast_FireBolt.AM_Cast_FireBolt"
        (:`then`
          (`AbilityTask_WaitGameplayEvent.WaitGameplayEvent` (struct :`TagName` "Event.Montage.FireBolt") null true
            (:`EventReceived`
              (`self.SpawnProjectile` (`KismetMathLibrary.MakeTransform` (0.0 0.0 0.0))))))
        (:`OnCompleted`
          (`self.K2_EndAbility` :!label _label))
        (:`OnInterrupted`
          (goto _label))
        (:`OnCancelled`
          (goto _label))))))